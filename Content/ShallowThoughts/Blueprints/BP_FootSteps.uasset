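; BP_FootSteps is an unfinished footstep component for FirstPersonCharacter; it plays no sound yet.
; Each tick it casts player character 0's owner, rather than the character itself, to FirstPersonCharacter, printing a warning on failure.
; Once its owner is beyond Stride from LastFootstepLocation while grounded, it runs a debug-drawn downward Visibility trace.
; The hit branch is empty and LastFootstepLocation is never updated.
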(event EventBeginPlay)

(event EventTick
  (params (DeltaSeconds :type Float%20%28single-precision%29))
  (bind _asfirst_person_character (Utilities|Casting|CastToFirstPersonCharacter (Components|GetOwner (Game|GetPlayerCharacter 0)))
    (:then
      (if (and (> (Math|Vector|VectorLength (- (Transformation|GetActorLocation (Components|GetOwner)) (Variables|Default|GetLastFootstepLocation))) (Variables|Default|GetStride)) (AI|Components|NavMovement|IsMovingonGround (Pawn|GetMovementComponent _asfirst_person_character)))
        (bind _asfirst_person_character_2 (Utilities|Casting|CastToFirstPersonCharacter (Components|GetOwner (Game|GetPlayerCharacter 0))))
        (bind _returnvalue (Collision|LineTraceByChannel (Transformation|GetActorLocation _asfirst_person_character_2) (- (Transformation|GetActorLocation _asfirst_person_character_2) (Math|Vector|MakeVector 0.0 0.0 (* (Components|Capsule|GetUnscaledCapsuleHalfHeight (Variables|/Script/Engine.Character|GetCapsuleComponent _asfirst_person_character_2)) 2.0))) "TraceTypeQuery1" false 0 "ForDuration"))
        (if _returnvalue
          _)))
    (:CastFailed
      (Development|PrintString "BP_FootSteps added to non-character Actor!"))))